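; Grid Blueprint for a Tetris game, with the visible graphs providing debug visualization of the grid and game state.
; The construction script flushes persistent debug lines, then draws a long-lived box at the world location of each TetrisGridMap key.
; Every tick prints level, completed rows, combo, points, last Tetris score and game speed to the screen only.
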(event `self.ReceiveTick`
  (params (DeltaSeconds :type "Float (single-precision)"))
  (`KismetSystemLibrary.PrintString` (`KismetStringLibrary.Concat_StrStr` " \ncurrent level:" (`KismetStringLibrary.Conv_IntToString` (`self.currentLevel`)) " \ncurrentCompletedRowCount:" (`KismetStringLibrary.Conv_IntToString` (`self.currentCompletedRowCount`)) " \ncurrentCombo:" (`KismetStringLibrary.Conv_IntToString` (`self.currentCombo`)) " \ncurrentPoints:" (`KismetStringLibrary.Conv_IntToString` (`self.currentPoints`)) " \nlastTetrisScore:" (`|GetEnumeratorNameAsString` (`self.lastTetrisScore`)) " \ncurrent speed:" (`KismetStringLibrary.Conv_DoubleToString` (`self.currentGameSpeed`))) true false (struct :`R` 0.936395 :`G` 0.277561 :`B` 1.0 :`A` 1.0) 0.0))

(fn `UserConstructionScript`
  (`KismetSystemLibrary.FlushPersistentDebugLines`)
  (bind _keys (`BlueprintMapLibrary.Map_Keys` (`self.tetrisGridMap`)))
  (for _array_element _keys
    (`KismetSystemLibrary.DrawDebugBox` (`self.ConverGridIndexToWorldLocation` _array_element) (10.0 10.0 10.0) (struct :`R` 0.522 :`G` 1.0 :`B` 0.223487 :`A` 1.0) (struct) 10000.0 0.05)))